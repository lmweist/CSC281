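; BP_Yeti is a 2D flipbook boss enemy that fights BP_SpriteCharacter once StartFight is called.
; Tick drives velocity, facing, animation, health and Think, which randomly picks a charge or three-snowball volley when the player is distant.
; Charges reverse on ExitBounds with a rising chance to stop.
; Hits cause a flash, brief invulnerability and knockback outside charges; death hides the actor for RespawnEnemy to restore.
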(event OnFinishedPlaying(Sprite)
  (Sprite|SetFlipbook (Variables|Default|GetSprite) "/Game/Sprites/Yeti/yetiRedoneIdle.yetiRedoneIdle")
  (Variables|Default|SetisAttacking false)
  (Development|SetHiddeninGame (Variables|Default|GetHitbox) true false))

(event Custom|UpdateAnimation
  (if (not (== (Class|PaperFlipbookComponent|GetFlipbook (Variables|Default|GetSprite)) "/Game/Maps/SunnyLandAssets/sprites/Santa2/Santa_Attack1_FB.Santa_Attack1_FB"))
    (Sprite|SetFlipbook (Variables|Default|GetSprite) (select (Variables|Default|GetinThrowingAttack) "/Game/Sprites/Yeti/yetiRedoneThrow.yetiRedoneThrow" (select (> (Math|Vector|VectorLength (Variables|Default|GetdesiredVelocity)) 1e+02) "/Game/Sprites/Yeti/yetiRedoneSprint.yetiRedoneSprint" (select (> (Math|Vector|VectorLength (Variables|Default|GetdesiredVelocity)) 0.0) "/Game/Sprites/Yeti/yetiRedoneWalking.yetiRedoneWalking" "/Game/Sprites/Yeti/yetiRedoneIdle.yetiRedoneIdle"))))))

(event Custom|UpdateControlRotation
  (Utilities|IsValid (Pawn|GetController)
    (:Is%20Valid
      (Math|Float|CompareFloat (.X (Math|Vector|BreakVector (Variables|Default|GetdesiredVelocity))) 0.0
        (:>
          (Transformation|SetActorRotation (Math|Rotator|MakeRotator 0.0 0.0 0.0)))
        (:<
          (Transformation|SetActorRotation (Math|Rotator|MakeRotator 0.0 0.0 1.8e+02)))))))

(event Custom|Think
  (Development|PrintString (Utilities|String|ToString(Boolean) (Variables|Default|GetperformingAttack)) true true "(R=0.000000,G=0.660000,B=1.000000,A=1.000000)" 4.0)
  (if (not (Variables|Default|GetperformingAttack))
    (Variables|Default|SetisThinking true)
    (bind _distance (CallFunction|GetDistancetoPlayer))
    (Development|PrintString (Utilities|String|ToString(Float) _distance))
    (if (> _distance 3e+02)
      (Development|PrintString "Far enough away...")
      (if (Math|Random|RandomBool)
        (Development|PrintString "True...")
        (bind _returnvalue (Actor|GetActorOfClass "/Game/Blueprints/BP_SpriteCharacter.BP_SpriteCharacter_C"))
        (Variables|Default|SetdesiredVelocity (Math|Vector|MakeVector (* (.X (Math|Vector|BreakVector (Class|KismetMathLibrary|VectorGetSignVector (- (Transformation|GetActorLocation _returnvalue) (Transformation|GetActorLocation))))) (Variables|Default|GetrunningAttackVelocity)) 0.0 0.0))
        (Variables|Default|SetinRunningAttack true)
        (Variables|Default|SetperformingAttack true)
        (Variables|Default|SetstopChance 0.5)
        (Variables|Default|SetisThinking (Variables|Default|Getfalse))
        (else
          (Variables|Default|SetperformingAttack true)
          (Variables|Default|SetinThrowingAttack true)
          (Sprite|SetFlipbook (Variables|Default|GetSprite) "/Game/Sprites/Yeti/yetiRedoneThrow.yetiRedoneThrow")
          (Game|SpawnActorfromClass "/Game/Blueprints/BP_Snowball.BP_Snowball_C" (Transformation|GetWorldTransform (Variables|Default|GetProjectileSpawnLocation)) "AlwaysSpawn" "MultiplyWithRoot" 0 0)
          (Utilities|FlowControl|Delay 0.3)
          (Sprite|SetFlipbook (Variables|Default|GetSprite) "/Game/Sprites/Yeti/yetiRedoneThrow.yetiRedoneThrow")
          (Game|SpawnActorfromClass "/Game/Blueprints/BP_Snowball.BP_Snowball_C" (Transformation|GetWorldTransform (Variables|Default|GetProjectileSpawnLocation)) "AlwaysSpawn" "MultiplyWithRoot" 0 0)
          (Utilities|FlowControl|Delay 0.3)
          (Sprite|SetFlipbook (Variables|Default|GetSprite) "/Game/Sprites/Yeti/yetiRedoneThrow.yetiRedoneThrow")
          (Game|SpawnActorfromClass "/Game/Blueprints/BP_Snowball.BP_Snowball_C" (Transformation|GetWorldTransform (Variables|Default|GetProjectileSpawnLocation)) "AlwaysSpawn" "MultiplyWithRoot" 0 0)
          (Utilities|FlowControl|Delay 0.3)
          (Variables|Default|SetisThinking false)
          (Variables|Default|SetinThrowingAttack false)
          (Variables|Default|SetperformingAttack false)))
      (else
        (Variables|Default|SetisThinking false)))))

(event Custom|RespawnEnemy
  (if (== 0.0 (Variables|Default|GetHealth))
    (Transformation|Teleport (Variables|Default|Getlocation) "0, 0, 0")
    (Rendering|SetActorHiddenInGame self false)
    (Collision|SetActorEnableCollision self true)
    (Development|PrintString "\"Spawning\"")
    (else
      (Development|PrintString (Utilities|String|ToString(Float) (Variables|Default|GetHealth)))))
  (Variables|Default|SetHealth (Variables|Default|GetMaxHealth)))

(event Custom|ExitBounds
  (if (Variables|Default|GetinRunningAttack)
    (if (>= (Variables|Default|GetstopChance) (Math|Random|RandomFloatinRange 0.0 0.999))
      (Variables|Default|SetdesiredVelocity (Math|Vector|MakeVector (* (.X (Math|Vector|BreakVector (Class|KismetMathLibrary|VectorGetSignVector (Variables|Default|GetdesiredVelocity)))) -1.0) 0.0 0.0))
      (Utilities|FlowControl|Delay 0.2)
      (Utilities|FlowControl|Delay 0.01)
      (Variables|Default|SetdesiredVelocity "0, 0, 0")
      (Variables|Default|SetperformingAttack false)
      (Variables|Default|SetinRunningAttack false)
      (else
        (Variables|Default|SetdesiredVelocity (* (Variables|Default|GetdesiredVelocity) "-1.000000,0.000000,0.000000"))
        (Variables|Default|SetstopChance (+ (Variables|Default|GetstopChance) 0.25))))
    (else
      (Variables|Default|SetdesiredVelocity (* (Variables|Default|GetdesiredVelocity) "-1.000000,0.000000,0.000000")))))

(event Custom|SetTheVelocity
  (if (not (AI|Components|NavMovement|IsFalling (Variables|Character|GetCharacterMovement)))
    (Variables|/Script/Engine.MovementComponent|SetVelocity (Variables|Character|GetCharacterMovement) (Variables|Default|GetdesiredVelocity))))

(event Custom|CheckHealth
  (if (not (> (Variables|Default|GetHealth) 0.0))
    (Rendering|SetActorHiddenInGame true)
    (Collision|SetActorEnableCollision self false)))

(event Custom|EnterBounds
  (if (== (Math|Vector|VectorLength (Variables|/Script/Engine.MovementComponent|GetVelocity (Variables|Character|GetCharacterMovement))) 0.0)
    (Variables|Default|SetdesiredVelocity "100.000000,0.000000,0.000000")))

(event Custom|StartFight
  (Variables|Default|SetfightStarted true)
  (Development|PrintString "Fight started"))

(event Custom|CallHitCheck
  (if (Variables|Default|GetisAttacking)
    (CallFunction|HitCheck)))

(event EventTick
  (params (DeltaSeconds :type Float%20%28single-precision%29))
  (if (Variables|Default|GetfightStarted)
    (CallFunction|CallHitCheck)
    (CallFunction|SettheVelocity)
    (CallFunction|UpdateControlRotation)
    (CallFunction|UpdateAnimation)
    (CallFunction|CheckHealth)
    (CallFunction|Think)))

(event EventBeginPlay
  (Variables|Default|Setlocation (Transformation|GetWorldLocation (Variables|Collision|GetCapsuleComponent))))

(event Game|Damage|EventAnyDamage
  (params (Damage :type Float%20%28single-precision%29) (DamageType :type Damage%20Type%20Object%20Reference) (InstigatedBy :type Controller%20Object%20Reference) (DamageCauser :type Actor%20Object%20Reference))
  (if (Variables|Default|GetcanBeAttacked)
    (Variables|Default|SetcanBeAttacked false)
    (Variables|Default|SetHealth (- (Variables|Default|GetHealth) Damage))
    (if (Variables|Default|GetinRunningAttack)
      _
      (else
        (Character|LaunchCharacter (+ (* (Class|KismetMathLibrary|VectorGetSignVector (- (Transformation|GetActorLocation) (Transformation|GetActorLocation DamageCauser))) "20.000000,0.000000,0.000000") "0.000000,0.000000,60.000000") true true)))
    (Rendering|Material|SetMaterial (Variables|Default|GetSprite) 0 "/Game/Blueprints/spriteDamage_Material2.spriteDamage_Material2")
    (Utilities|FlowControl|Delay 0.2)
    (Rendering|Material|SetMaterial (Variables|Default|GetSprite) 0 "/Game/Blueprints/sprite_Material.sprite_Material")
    (Utilities|FlowControl|Delay 0.3)
    (Variables|Default|SetcanBeAttacked true)))

(fn ConstructionScript)

(fn RestartAnim
  (Components|Timeline|SetLooping (Variables|Default|GetSprite) false)
  (if (not (Audio|Components|Audio|IsPlaying (Variables|Default|GetSprite)))
    (Audio|Components|Audio|Play (Variables|Default|GetSprite))))

(fn HitCheck
  (for _array_element (Collision|GetOverlappingActors (Variables|Default|GetHitbox) "/Game/Blueprints/BP_SpriteCharacter.BP_SpriteCharacter_C" :!class /Script/Engine.PrimitiveComponent)
    (Development|PrintString (Utilities|GetDisplayName _array_element) true true "(R=0.946939,G=0.000000,B=1.000000,A=1.000000)")
    (if (!= _array_element self)
      (if (Variables|Default|GetisAttacking)
        (Game|Damage|ApplyDamage _array_element (Variables|Default|GetDamageAmount) 0 self "/Script/Engine.DamageType")))))

(fn GetDistancetoPlayer
  (bind _returnvalue (Actor|GetActorOfClass "/Game/Blueprints/BP_SpriteCharacter.BP_SpriteCharacter_C"))
  (return (Math|Vector|Distance(Vector) (Transformation|GetActorLocation _returnvalue) (Transformation|GetActorLocation))))