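; Mrs. Claus sprite character that shows an interaction widget while the player's Santa sprite character is nearby.
; It creates the P_MrsClaus widget on BeginPlay, then Hitbox overlaps with BP_SpriteCharacter add or remove it and set the SantaOverlapping flag.
; RestartAnim and HitCheck helpers replay the sprite without looping and damage other actors in the same Hitbox, but nothing here calls them.
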(event OnComponentBeginOverlap(Hitbox)
  (params (OverlappedComponent :type Primitive%20Component%20Object%20Reference) (OtherActor :type Actor%20Object%20Reference) (OtherComp :type Primitive%20Component%20Object%20Reference) (OtherBodyIndex :type Integer) (bFromSweep :type Boolean) (SweepResult :type Hit%20Result%20Structure%20%28by%20ref%29))
  (bind _returnvalue (Actor|GetActorOfClass "/Game/Blueprints/BP_SpriteCharacter.BP_SpriteCharacter_C"))
  (if (== OtherActor _returnvalue)
    (UserInterface|Viewport|AddtoViewport (Variables|Default|GetinteractWidget) 0)
    (Variables|Default|SetsantaOverlapping true)))

(event OnComponentEndOverlap(Hitbox)
  (params (OverlappedComponent :type Primitive%20Component%20Object%20Reference) (OtherActor :type Actor%20Object%20Reference) (OtherComp :type Primitive%20Component%20Object%20Reference) (OtherBodyIndex :type Integer))
  (bind _returnvalue (Actor|GetActorOfClass "/Game/Blueprints/BP_SpriteCharacter.BP_SpriteCharacter_C"))
  (if (== _returnvalue OtherActor)
    (Widget|RemovefromParent (Variables|Default|GetinteractWidget))
    (Variables|Default|SetsantaOverlapping false)))

(event EventBeginPlay
  (bind _returnvalue (UserInterface|CreateWidget "/Game/Widgets/P_MrsClaus.P_MrsClaus_C"))
  (Variables|Default|SetinteractWidget _returnvalue))

(fn ConstructionScript)

(fn RestartAnim
  (Components|Timeline|SetLooping (Variables|Default|GetSprite) false)
  (if (not (Audio|Components|Audio|IsPlaying (Variables|Default|GetSprite)))
    (Audio|Components|Audio|Play (Variables|Default|GetSprite))))

(fn HitCheck
  (for _array_element (Collision|GetOverlappingActors (Variables|Default|GetHitbox) 0 :!class /Script/Engine.PrimitiveComponent)
    (if (!= _array_element self)
      (Game|Damage|ApplyDamage _array_element (Variables|Default|GetDamageAmount) 0 0))))