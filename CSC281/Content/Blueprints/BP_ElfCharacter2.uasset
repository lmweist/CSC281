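; Paper2D evil elf enemy that patrols horizontally, reversing direction through bounds events that are called externally.
; Tick drives velocity, facing, flipbook and health checks; death hides the elf and reports the kill once to BP_SpriteCharacter.
; Damage causes knockback, a material flash and brief invulnerability, while respawn restores it at its start location.
; A hitbox overlap attack exists, but the nodes that start it are unwired.
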(event OnFinishedPlaying(Sprite)
  (Sprite|SetFlipbook (Variables|Default|GetSprite) "/Game/Sprites/Elf/EvilElfIdle.EvilElfIdle")
  (Variables|Default|SetisAttacking false)
  (Development|SetHiddeninGame (Variables|Default|GetHitbox) true false))

(event Custom|UpdateAnimation
  (if (not (== (Class|PaperFlipbookComponent|GetFlipbook (Variables|Default|GetSprite)) "/Game/Maps/SunnyLandAssets/sprites/Santa2/Santa_Attack1_FB.Santa_Attack1_FB"))
    (Sprite|SetFlipbook (Variables|Default|GetSprite) (select (AI|Components|NavMovement|IsFalling (Variables|Character|GetCharacterMovement)) "/Game/Sprites/Elf/EvilElfIdle.EvilElfIdle" (select (> (Math|Vector|VectorLength (Variables|Default|GetdesiredVelocity)) 0.0) "/Game/Sprites/Elf/EvilElfWalking.EvilElfWalking" "/Game/Sprites/Elf/EvilElfIdle.EvilElfIdle")))))

(event Custom|UpdateControlRotation
  (Utilities|IsValid (Pawn|GetController)
    (:Is%20Valid
      (Math|Float|CompareFloat (.X (Math|Vector|BreakVector (Variables|Default|GetdesiredVelocity))) 0.0
        (:>
          (Transformation|SetActorRotation (Math|Rotator|MakeRotator 0.0 0.0 1.8e+02)))
        (:<
          (Transformation|SetActorRotation (Math|Rotator|MakeRotator 0.0 0.0 0.0)))))))

(event Custom|RespawnEnemy
  (Transformation|Teleport (Variables|Default|Getlocation) "0, 0, 0")
  (if (<= (Variables|Default|GetHealth) 0.0)
    (Rendering|SetActorHiddenInGame self false)
    (Collision|SetActorEnableCollision self true)
    (Variables|Default|SetaddedXP false))
  (Variables|Default|SetHealth (Variables|Default|GetMaxHealth)))

(event Custom|ExitBounds
  (Variables|Default|SetdesiredVelocity (* (Variables|Default|GetdesiredVelocity) "-1.000000,0.000000,0.000000")))

(event Custom|FallingOffMap
  (Rendering|SetActorHiddenInGame true)
  (Collision|SetActorEnableCollision self false)
  (Transformation|Teleport (Variables|Default|Getlocation) "0, 0, 0")
  (Variables|Default|SetHealth 0.0))

(event Custom|SetTheVelocity
  (if (not (AI|Components|NavMovement|IsFalling (Variables|Character|GetCharacterMovement)))
    (Variables|/Script/Engine.MovementComponent|SetVelocity (Variables|Character|GetCharacterMovement) (Variables|Default|GetdesiredVelocity))))

(event Custom|CheckHealth
  (if (not (> (Variables|Default|GetHealth) 0.0))
    (Rendering|SetActorHiddenInGame true)
    (Collision|SetActorEnableCollision self false)
    (if (not (Variables|Default|GetaddedXP))
      (bind _returnvalue (Actor|GetActorOfClass "/Game/Blueprints/BP_SpriteCharacter.BP_SpriteCharacter_C"))
      (Default|OnElfKill2 _returnvalue)
      (Variables|Default|SetaddedXP true))))

(event Custom|EnterBounds
  (if (== (Math|Vector|VectorLength (Variables|/Script/Engine.MovementComponent|GetVelocity (Variables|Character|GetCharacterMovement))) 0.0)
    (Variables|Default|SetdesiredVelocity "100.000000,0.000000,0.000000")))

(event Custom|CallHitCheck
  (if (Variables|Default|GetisAttacking)
    (CallFunction|HitCheck)))

(event EventTick
  (params (DeltaSeconds :type Float%20%28single-precision%29))
  (CallFunction|CallHitCheck)
  (CallFunction|SettheVelocity)
  (CallFunction|UpdateControlRotation)
  (CallFunction|UpdateAnimation)
  (CallFunction|CheckHealth))

(event EventBeginPlay
  (Variables|Default|Setlocation (Transformation|GetWorldLocation (Variables|Collision|GetCapsuleComponent)))
  (Utilities|FlowControl|Delay 0.5)
  (Variables|Default|SetdesiredVelocity "100.000000,0.000000,0.000000"))

(event Game|Damage|EventAnyDamage
  (params (Damage :type Float%20%28single-precision%29) (DamageType :type Damage%20Type%20Object%20Reference) (InstigatedBy :type Controller%20Object%20Reference) (DamageCauser :type Actor%20Object%20Reference))
  (if (Variables|Default|GetcanBeAttacked)
    (Audio|PlaySound2D "/Game/Sounds/damagesound/ManHurt.ManHurt" 1.0 1.0 0.0 0 0)
    (Variables|Default|SetcanBeAttacked false)
    (Variables|Default|SetHealth (- (Variables|Default|GetHealth) Damage))
    (Character|LaunchCharacter (+ (* (Class|KismetMathLibrary|VectorGetSignVector (- (Transformation|GetActorLocation) (Transformation|GetActorLocation DamageCauser))) "66.000000,0.000000,0.000000") "0.000000,0.000000,200.000000") true true)
    (Rendering|Material|SetMaterial (Variables|Default|GetSprite) 0 "/Game/Blueprints/spriteDamage_Material2.spriteDamage_Material2")
    (Utilities|FlowControl|Delay 0.2)
    (Rendering|Material|SetMaterial (Variables|Default|GetSprite) 0 "/Game/Blueprints/sprite_Material.sprite_Material")
    (Utilities|FlowControl|Delay 0.3)
    (Variables|Default|SetcanBeAttacked true)))

(fn ConstructionScript)

(fn RestartAnim
  (Components|Timeline|SetLooping (Variables|Default|GetSprite) false)
  (if (not (Audio|Components|Audio|IsPlaying (Variables|Default|GetSprite)))
    (Audio|Components|Audio|Play (Variables|Default|GetSprite))))

(fn HitCheck
  (for _array_element (Collision|GetOverlappingActors (Variables|Default|GetHitbox) "/Game/Blueprints/BP_SpriteCharacter.BP_SpriteCharacter_C" :!class /Script/Engine.PrimitiveComponent)
    (if (!= _array_element self)
      (if (Variables|Default|GetisAttacking)
        (Game|Damage|ApplyDamage _array_element (Variables|Default|GetDamageAmount) 0 self "/Script/Engine.DamageType")))))