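; BP_ReindeerCharacter2 is a reindeer character with a sprite and a hitbox for dealing and receiving damage.
; RestartAnim turns off sprite looping and replays the animation if it has stopped.
; HitCheck applies DamageAmount to every other actor overlapping the Hitbox.
; Incoming damage is only printed to screen in green, with no health handling in this Blueprint.
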(event Game|Damage|EventAnyDamage
  (params (Damage :type Float%20%28single-precision%29) (DamageType :type Damage%20Type%20Object%20Reference) (InstigatedBy :type Controller%20Object%20Reference) (DamageCauser :type Actor%20Object%20Reference))
  (Development|PrintString (Utilities|String|ToString(Float) Damage) true true "(R=0.000000,G=1.000000,B=0.154189,A=1.000000)"))

(fn ConstructionScript)

(fn RestartAnim
  (Components|Timeline|SetLooping (Variables|Default|GetSprite) false)
  (if (not (Audio|Components|Audio|IsPlaying (Variables|Default|GetSprite)))
    (Audio|Components|Audio|Play (Variables|Default|GetSprite))))

(fn HitCheck
  (for _array_element (Collision|GetOverlappingActors (Variables|Default|GetHitbox) 0 :!class /Script/Engine.PrimitiveComponent)
    (if (!= _array_element self)
      (Game|Damage|ApplyDamage _array_element (Variables|Default|GetDamageAmount) 0 0))))