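; BP_Snowball is a short-lived snowball actor that damages any BP_SpriteCharacter it touches.
; Each tick it polls its Hitbox for overlapping characters, applies damage to every one found, then destroys itself if any were hit.
; It also destroys itself on a Hit event, after a fixed lifetime, or when it falls to a set world height.
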(event Custom|Call%20Hit%20Check
  (Utilities|IsValid (Variables|Default|GetHitbox)
    (:Is%20Valid
      (CallFunction|HitCheck)
      (Utilities|IsValid (Variables|Default|GetHitbox)
        (:Is%20Valid
          (if (<= (.Z (Math|Vector|BreakVector (Transformation|GetActorLocation))) -3.2e+02)
            (Actor|DestroyActor)))))))

(event EventTick
  (params (DeltaSeconds :type Float%20%28single-precision%29))
  (CallFunction|CallHitCheck))

(event Collision|EventHit
  (params (MyComp :type Primitive%20Component%20Object%20Reference) (Other :type Actor%20Object%20Reference) (OtherComp :type Primitive%20Component%20Object%20Reference) (bSelfMoved :type Boolean) (HitLocation :type Vector :default "0, 0, 0") (HitNormal :type Vector :default "0, 0, 0") (NormalImpulse :type Vector :default "0, 0, 0") (Hit :type Hit%20Result%20Structure%20%28by%20ref%29))
  (Actor|DestroyActor))

(event EventBeginPlay
  (Utilities|FlowControl|Delay 5.0)
  (Actor|DestroyActor))

(fn ConstructionScript)

(fn HitCheck
  (bind _hitbox (Variables|Default|GetHitbox))
  (Variables|Default|SetsnowballHitPlayer false)
  (Utilities|IsValid _hitbox
    (:Is%20Valid
      (for _array_element (Collision|GetOverlappingActors _hitbox "/Game/Blueprints/BP_SpriteCharacter.BP_SpriteCharacter_C" :!class /Script/Engine.PrimitiveComponent)
        (Game|Damage|ApplyDamage _array_element (Variables|Default|GetDamageAmount) 0 self "/Script/Engine.DamageType")
        (Variables|Default|SetsnowballHitPlayer true))
      (if (Variables|Default|GetsnowballHitPlayer)
        (Actor|DestroyActor)))))